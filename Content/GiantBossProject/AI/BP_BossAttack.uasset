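; BP_BossAttack is a behavior tree task that makes the BP_Giant boss perform an attack.
; It measures the giant's distance to the player and plays a random montage from a short-range or long-range set, split at a fixed threshold.
; The task succeeds when the montage completes, and fails if it is interrupted or the controlled pawn is not a BP_Giant.
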(event EventReceiveExecuteAI
  (params (OwnerController :type AI%20Controller%20Object%20Reference) (ControlledPawn :type Pawn%20Object%20Reference))
  (bind _asbp_giant (Utilities|Casting|CastToBP_Giant ControlledPawn)
    (:then
      (Variables|Default|Setintermediate_distance (Math|Vector|VectorLength (- (Transformation|GetActorLocation _asbp_giant) (Transformation|GetActorLocation (Game|Player|GetPlayerPawn 0)))))
      (if (<= (Variables|Default|Getintermediate_distance) 7e+02)
        (Animation|Montage|PlayMontage (Variables|/Script/Engine.Character|GetMesh _asbp_giant) (.OutItem (Utilities|Array|Random (Variables|Default|GetMontage%20to%20Play_Short)))
          (:OnCompleted
            (AI|BehaviorTree|FinishExecute true :!label _label))
          (:OnInterrupted
            (AI|BehaviorTree|FinishExecute false :!label _label_2)))
        (else
          (Animation|Montage|PlayMontage (Variables|/Script/Engine.Character|GetMesh _asbp_giant) (.OutItem (Utilities|Array|Random (Variables|Default|GetMontage%20to%20Play_Long)))
            (:OnCompleted
              (goto _label))
            (:OnInterrupted
              (goto _label_2))))))
    (:CastFailed
      (goto _label_2))))